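; Player character Blueprint for a sponge, which shows how much it has absorbed through its material.
; BeginPlay creates a dynamic M_Frankensponge instance on the Model, and Tick feeds PercentAbsorbed into its Wetness parameter every frame.
; The release-hold binding and the test liquid-field SpongeRelease call are disconnected, and the overlap and release event handlers are empty.
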(event Custom|OnReleaseHold_Event
  (params (DeltaTime :type Float%20%28single-precision%29)))

(event EventBeginPlay
  (bind _returnvalue (Rendering|Material|CreateDynamicMaterialInstance (Variables|Default|GetModel) 0 "/Game/Models/Frankensponge/M_Frankensponge.M_Frankensponge" "None" :!class /Script/Engine.PrimitiveComponent))
  (Variables|Default|SetSpongeMaterial _returnvalue))

(event EventTick
  (params (DeltaSeconds :type Float%20%28single-precision%29))
  (Rendering|Material|SetScalarParameterValue (Variables|Default|GetSpongeMaterial) "Wetness" (Variables|Default|GetPercentAbsorbed) :!class /Script/Engine.MaterialInstanceDynamic))

(event Collision|EventActorBeginOverlap
  (params (OtherActor :type Actor%20Object%20Reference)))

(event Collision|EventActorEndOverlap
  (params (OtherActor :type Actor%20Object%20Reference)))

(fn ConstructionScript)