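; Test actor for a sponge mechanic in which the player absorbs or releases Niagara particles by shrinking or growing them.
; The InputOutput system exports particle data to this actor, which checks whether the player's BoundingBox overlaps its Box.
; SpongeAbsorb (sphere overlap) and SpongeRelease (point-in-box) resize particles within that BoundingBox and write sizes back through the Import array.
; The total size change goes to the player's Absorb or Release.
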(event EventBeginPlay
  (Class|NiagaraComponent|SetVariableObject (Variables|Default|GetInputOutput) "PosExport" self))

(event Collision|EventActorBeginOverlap
  (params (OtherActor :type Actor%20Object%20Reference)))

(event EventTick
  (params (DeltaSeconds :type Float%20%28single-precision%29)))

(event EventParticleData
  (params (Data :type Array%20of%20Basic%20Particle%20Data%20Structures) (NiagaraSystem :type Niagara%20System%20Object%20Reference) (SimulationPositionOffset :type Vector%20%28by%20ref%29 :default "0, 0, 0"))
  (Variables|Default|SetData Data)
  (bind _asbp_new_char_player (Utilities|Casting|CastToBP_NewCharPlayer (Game|Player|GetPlayerPawn 0)))
  (if (and (Variables|/Script/Frankensponge.CharPlayer|GetbIsReleasing _asbp_new_char_player) (Class|PrimitiveComponent|IsOverlappingComponent (Variables|/Script/Frankensponge.CharPlayer|GetBoundingBox _asbp_new_char_player) (Variables|Default|GetBox)))
    (bind _released (CallFunction|SpongeRelease (Variables|/Script/Frankensponge.CharPlayer|GetBoundingBox _asbp_new_char_player)))
    (Class|CharPlayer|Release _asbp_new_char_player _released)
    (elif (and (Class|PrimitiveComponent|IsOverlappingComponent (Variables|/Script/Frankensponge.CharPlayer|GetBoundingBox _asbp_new_char_player) (Variables|Default|GetBox)) (Variables|/Script/Frankensponge.CharPlayer|GetbIsAbsorbing _asbp_new_char_player))
      (bind _absorb (CallFunction|SpongeAbsorb (Variables|/Script/Frankensponge.CharPlayer|GetBoundingBox _asbp_new_char_player)))
      (Class|CharPlayer|Absorb _asbp_new_char_player _absorb))))

(fn ConstructionScript)

(fn SpongeRelease
  (params (SpongeCollision :type Box%20Component%20Object%20Reference))
  (bind _returnvalue (Utilities|Time|GetWorldDeltaSeconds))
  (bind _datavec2 (Variables|Default|GetDataVec2))
  (bind _datavec2_2 (Variables|Default|GetDataVec2))
  (LocalVariables|SetTotalRelease 0.0)
  (if (> (Variables|Default|GetPreTime) 0.0)
    (Variables|Default|SetPreTime (- _returnvalue (Variables|Default|GetPreTime)))
    (else
      (Variables|Default|SetTimer _returnvalue)))
  (Utilities|Array|Clear _datavec2)
  (for _array_element (Variables|Default|GetData)
    (if (Class|KismetMathLibrary|IsPointinBoxwithTransform (.Position (Utilities|Struct|BreakBasicParticleData _array_element)) (Transformation|GetWorldTransform SpongeCollision) (* (Transformation|GetWorldScale SpongeCollision) "30.000000,30.000000,30.000000"))
      (Utilities|Array|Add _datavec2_2 (Math|Vector2D|MakeVector2D (Math|Float|Clamp(Float) (+ (.Size (Utilities|Struct|BreakBasicParticleData _array_element)) (* (Variables|Default|GetTimer) 1e+02)) 0.0 5e+01) (Math|Float|Clamp(Float) (+ (.Size (Utilities|Struct|BreakBasicParticleData _array_element)) (* (Variables|Default|GetTimer) 1e+02)) 0.0 5e+01)))
      (LocalVariables|SetTotalRelease (+ (- (Math|Float|Clamp(Float) (+ (.Size (Utilities|Struct|BreakBasicParticleData _array_element)) (* (Variables|Default|GetTimer) 1e+02)) 0.0 5e+01) (.Size (Utilities|Struct|BreakBasicParticleData _array_element))) (LocalVariables|GetTotalRelease)))
      (else
        (Utilities|Array|Add _datavec2_2 (Math|Vector2D|MakeVector2D (.Size (Utilities|Struct|BreakBasicParticleData _array_element)) (.Size (Utilities|Struct|BreakBasicParticleData _array_element)))))))
  (Class|NiagaraDataInterfaceArrayFunctionLibrary|SetNiagaraArrayVector2D (Variables|Default|GetInputOutput) "Import" _datavec2)
  (return (LocalVariables|GetTotalRelease)))

(fn SpongeAbsorb
  (params (SpongeCollision :type Box%20Component%20Object%20Reference))
  (bind _returnvalue (Utilities|Time|GetWorldDeltaSeconds))
  (bind _datavec2 (Variables|Default|GetDataVec2))
  (bind _datavec2_2 (Variables|Default|GetDataVec2))
  (LocalVariables|SetTotalAbsorb 0.0)
  (if (> (Variables|Default|GetPreTime) 0.0)
    (Variables|Default|SetPreTime (- _returnvalue (Variables|Default|GetPreTime)))
    (else
      (Variables|Default|SetTimer _returnvalue)))
  (Utilities|Array|Clear _datavec2)
  (for _array_element (Variables|Default|GetData)
    (bind _returnvalue_2 (Class|PrimitiveComponent|SphereOverlapComponent SpongeCollision (.Position (Utilities|Struct|BreakBasicParticleData _array_element)) (.Size (Utilities|Struct|BreakBasicParticleData _array_element)) false false false))
    (if _returnvalue_2
      (Utilities|Array|Add _datavec2_2 (Math|Vector2D|MakeVector2D (Math|Float|Clamp(Float) (+ (.Size (Utilities|Struct|BreakBasicParticleData _array_element)) (* (Variables|Default|GetTimer) -1e+02)) 0.0 5e+01) (Math|Float|Clamp(Float) (+ (.Size (Utilities|Struct|BreakBasicParticleData _array_element)) (* (Variables|Default|GetTimer) -1e+02)) 0.0 5e+01)))
      (LocalVariables|SetTotalAbsorb (+ (- (.Size (Utilities|Struct|BreakBasicParticleData _array_element)) (Math|Float|Clamp(Float) (+ (.Size (Utilities|Struct|BreakBasicParticleData _array_element)) (* (Variables|Default|GetTimer) -1e+02)) 0.0 5e+01)) (LocalVariables|GetTotalAbsorb)))
      (else
        (Utilities|Array|Add _datavec2_2 (Math|Vector2D|MakeVector2D (.Size (Utilities|Struct|BreakBasicParticleData _array_element)) (.Size (Utilities|Struct|BreakBasicParticleData _array_element)))))))
  (Class|NiagaraDataInterfaceArrayFunctionLibrary|SetNiagaraArrayVector2D (Variables|Default|GetInputOutput) "Import" _datavec2)
  (return (LocalVariables|GetTotalAbsorb)))